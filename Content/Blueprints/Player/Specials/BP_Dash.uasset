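; BP_Dash is a player special that briefly boosts the owning character along its movement input, or straight forward when there is none.
; Activate saves walk speed, ground friction and acceleration, multiplies speed by SpeedModifier, removes friction and raises acceleration.
; A timeline, started partway through so DashDuration sets its remaining length, feeds movement input every update.
; When the timeline finishes, FinishActivate restores the saved movement values.
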(event `Dash`
  (params (Direction :type "Vector Structure"))
  (`TimelineComponent.SetPlaybackPosition` (`self.DashTimeline`) (- 1.0 (`self.DashDuration`)) false false)
  (`Timeline|DashTimeline` :`NewTime` 0.0
    (:`Update`
      (`Pawn.AddMovementInput` (`self.MyOwningCharacter`) (select `bool` (== (`KismetMathLibrary.VSizeSquared` Direction) 0.0) :`false` Direction :`true` (`self.GetActorForwardVector` (`self.MyOwningCharacter`))) 1.0 false))
    (:`Finished`
      (`self.FinishActivate`))))

(fn `Activate`
  (bind _myowningcharacter (`self.MyOwningCharacter`))
  (bind _charactermovement (`Character.CharacterMovement` (`self.MyOwningCharacter`)))
  (bind _charactermovement_2 (`Character.CharacterMovement` (`self.MyOwningCharacter`)))
  (`parent.Activate`)
  (bind _output_get (set `self.PreviousWalkSpeed` (`/Game/Blueprints/Player/BP_PlayerCharacter.MaxWalkSpeed` (`self.MyOwningCharacter`))))
  (set `CharacterMovementComponent.MaxWalkSpeed` (* _output_get (`self.SpeedModifier`)) (`Character.CharacterMovement` (`self.MyOwningCharacter`)))
  (set `self.PreviousFriction` (`CharacterMovementComponent.GroundFriction` _charactermovement))
  (set `CharacterMovementComponent.GroundFriction` 0.0 _charactermovement)
  (set `self.PreviousAcceleration` (`CharacterMovementComponent.MaxAcceleration` _charactermovement_2))
  (set `CharacterMovementComponent.MaxAcceleration` 10000.0 _charactermovement_2)
  (bind _asbp_player_controller (cast `/Game/Blueprints/Player/BP_PlayerController` (`Pawn.GetController` (`self.MyOwningCharacter`))))
  (`self.Dash` (+ (* (`self.GetActorForwardVector` _myowningcharacter) (`/Game/Blueprints/Player/BP_PlayerController.MyMoveForwardAxis` _asbp_player_controller)) (* (`self.GetActorRightVector` _myowningcharacter) (`/Game/Blueprints/Player/BP_PlayerController.MyMoveRightAxis` _asbp_player_controller)))))

(fn `FinishActivate`
  (bind _charactermovement (`Character.CharacterMovement` (`self.MyOwningCharacter`)))
  (set `CharacterMovementComponent.MaxWalkSpeed` (`self.PreviousWalkSpeed`) _charactermovement)
  (set `CharacterMovementComponent.GroundFriction` (`self.PreviousFriction`) _charactermovement)
  (set `CharacterMovementComponent.MaxAcceleration` (`self.PreviousAcceleration`) _charactermovement)
  (`parent.FinishActivate`))

(fn `UserConstructionScript`
  (`parent.UserConstructionScript`))