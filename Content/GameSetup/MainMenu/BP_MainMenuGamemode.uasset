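; Main menu game mode that sets up the menu HUD when play begins.
; On BeginPlay it spawns a BP_MainMenuHUD actor, stores the reference and turns split screen off.
; It then loops over its player controllers, casting each to BP_MenuController to initialize that controller's HUD.
; The parent BeginPlay is called twice, before the HUD spawn and again before the controller loop.
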(event `self.ReceiveBeginPlay`
  (`parent.ReceiveBeginPlay`)
  (bind _returnvalue (`|SpawnActorFromClass` "/Game/GameSetup/MainMenu/BP_MainMenuHUD.BP_MainMenuHUD_C" (`KismetMathLibrary.MakeTransform` (0.0 0.0 0.0)) "Undefined" "OverrideRootScale" null null))
  (set `self.MainMenuHUD` _returnvalue)
  (`self.ToggleSplitScreen` false)
  (`parent.ReceiveBeginPlay`)
  (for _array_element (`self.PlayerControllers`)
    (bind _asbp_menu_controller (cast `/Game/Blueprints/Player/BP_MenuController` _array_element))
    (`/Game/Blueprints/Player/BP_MenuController.InitializeHUD` _asbp_menu_controller)))

(fn `UserConstructionScript`
  (`parent.UserConstructionScript`))