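; State machine that drives a slime's movement through Idle, Wander and Flee states.
; A re-armed timer runs each state's exit check: Idle randomly starts Wander, Wander ends when the slime stops, Flee ends when no player is nearby.
; Wander moves toward random points, while Flee moves directly away from a nearby player, each at its own speed.
; No transition into Flee occurs within these graphs.
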(fn `AttemptLeaveFlee`
  (if (not (`.ReturnValue` (`/Game/Blueprints/Slime/BP_Slime.IsPlayerNearby` (`self.OwningSlime`) 500.0)))
    (`self.ChangeState` "NewEnumerator0")
    (else
      (`self.OnFlee`))))

(fn `AttemptLeaveIdle`
  (if (`KismetMathLibrary.RandomBoolWithWeight` 0.6)
    (`self.ChangeState` "NewEnumerator1")))

(fn `AttemptLeaveWander`
  (if (== (`KismetMathLibrary.VSizeSquared` (`MovementComponent.Velocity` (`Pawn.GetMovementComponent` (`self.OwningSlime`)))) 0.0)
    (`self.ChangeState` "NewEnumerator0")
    (`self.AttemptToChangeState`)))

(fn `AttemptToChangeState`
  (`/Engine/EditorBlueprintResources/StandardMacros.IsValid` (`self.OwningSlime`)
    (:`Is Valid`
      (`KismetSystemLibrary.K2_InvalidateTimerHandle` (`self.ChangeStateTimer`))
      (bind _returnvalue (`KismetSystemLibrary.K2_SetTimerDelegate` (`|CreateDelegate` :!event `AttemptToChangeState`) (`self.StateChangeInterval`)))
      (set `self.ChangeStateTimer` _returnvalue)
      (switch `/Game/Blueprints/Slime/ESlimeState` (`self.CurrentState`)
        (:`NewEnumerator0`
          (`self.AttemptLeaveIdle`))
        (:`NewEnumerator1`
          (`self.AttemptLeaveWander`))
        (:`NewEnumerator2`
          (`self.AttemptLeaveFlee`))))))

(fn `ChangeState`
  (params (NewState :type "/Game/Blueprints/Slime/ESlimeState Enum" :default "NewEnumerator0"))
  (if (!= NewState (`self.CurrentState`))
    (set `self.CurrentState` NewState)
    (`self.OnStateChanged`)
    (return)
    (else
      (return))))

(fn `OnFlee`
  (locals (FleeSpeed :type "Float (double-precision)" :default 500.0))
  (bind (_outactors _returnvalue) (`/Game/Blueprints/Slime/BP_Slime.IsPlayerNearby` (`self.OwningSlime`) 500.0))
  (if _returnvalue
    (set `CharacterMovementComponent.MaxWalkSpeed` (`local.FleeSpeed`) (`Character.CharacterMovement` (`self.OwningSlime`)))
    (`/Game/Blueprints/Slime/BP_SlimePawn.MoveToLocation` (`self.OwningSlime`) (+ (`Actor.K2_GetActorLocation` (`self.OwningSlime`)) (* (`KismetMathLibrary.Vector_Normal2D` (- (`Actor.K2_GetActorLocation` (`self.OwningSlime`)) (`Actor.K2_GetActorLocation` (`|GetArrayItem` _outactors)))) (`KismetMathLibrary.RandomFloatInRange` 800.0 1200.0))))
    (return)
    (else
      (`self.AttemptToChangeState`)
      (return))))

(fn `OnIdle`)

(fn `OnStateChanged`
  (switch `/Game/Blueprints/Slime/ESlimeState` (`self.CurrentState`)
    (:`NewEnumerator0`
      (`self.OnIdle`))
    (:`NewEnumerator1`
      (`self.OnWander`))
    (:`NewEnumerator2`
      (`self.OnFlee`)))
  (return))

(fn `OnWander`
  (locals (WanderSpeed :type "Float (double-precision)" :default 200.0))
  (set `CharacterMovementComponent.MaxWalkSpeed` (`local.WanderSpeed`) (`Character.CharacterMovement` (`self.OwningSlime`)))
  (`/Game/Blueprints/Slime/BP_SlimePawn.MoveToLocation` (`self.OwningSlime`) (+ (`Actor.K2_GetActorLocation` (`self.OwningSlime`)) (* (`KismetMathLibrary.RotateAngleAxis` (`Actor.GetActorForwardVector` (`self.OwningSlime`)) (* (`KismetMathLibrary.RandomFloat`) 360.0) (0.0 0.0 1.0)) (`KismetMathLibrary.RandomFloatInRange` 300.0 800.0)))))