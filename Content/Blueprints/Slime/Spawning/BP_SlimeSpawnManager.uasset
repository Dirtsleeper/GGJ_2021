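; BP_SlimeSpawnManager supplies random slime spawn points inside its box component volumes and registers itself with BP_Gamemode.
; On BeginPlay it disables each box's collision, caches its bounds and XY extent product as area, and accumulates a total.
; GetSpawnPoints splits the requested count across boxes in proportion to area, picking random points in each box's bounds.
; Per-box rounding makes the returned count approximate.
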(event `self.ReceiveBeginPlay`
  (for _array_element (`self.K2_GetComponentsByClass` "/Script/Engine.BoxComponent")
    (`PrimitiveComponent.SetCollisionEnabled` _array_element "NoCollision")
    (bind (_origin _boxextent) (`KismetSystemLibrary.GetComponentBounds` _array_element))
    (bind _returnvalue (* (.x _boxextent) (.y _boxextent)))
    (`BlueprintMapLibrary.Map_Add` (`self.MyComponents`) _array_element (make `/Game/Blueprints/Slime/Spawning/SpawnBounds` _origin (`KismetMathLibrary.MakeVector` (.x _boxextent) (.y _boxextent) (.z _boxextent)) _returnvalue))
    (set `self.TotalArea` (+ (`self.TotalArea`) _returnvalue))
    (bind _asbp_gamemode (cast `/Game/GameSetup/BP_GameMode` (`GameplayStatics.GetGameMode`)))
    (`/Game/GameSetup/BP_GameMode.SetSlimeSpawnManager` _asbp_gamemode self)))

(fn `GetSpawnPoints`
  (params (NumPoints :type Integer))
  (returns (Points :type "Array of Vector Structure"))
  (locals (PointsPerComponent :type Integer) (AreaPerPoint :type "Float (double-precision)" :default 0.0) (OutPoints :type "Array of Vector Structure") (CurrentSpawnBounds :type "/Game/Blueprints/Slime/Spawning/SpawnBounds Structure"))
  (bind (_currentspawnbounds_origin _currentspawnbounds_bounds) (break `/Game/Blueprints/Slime/Spawning/SpawnBounds` (`local.CurrentSpawnBounds`)))
  (set `local.AreaPerPoint` (/ (`self.TotalArea`) (`KismetMathLibrary.Conv_IntToDouble` NumPoints)))
  (bind _keys (`BlueprintMapLibrary.Map_Keys` (`self.MyComponents`)))
  (for _array_element _keys
    (bind _output_get (set `local.CurrentSpawnBounds` (`BlueprintMapLibrary.Map_Find` (`self.MyComponents`) _array_element)))
    (for _ (range (+ (`KismetMathLibrary.FFloor` (/ (`.Area_8_02A46ABF42829DDD7A3FE78C1A7050FB` (break `/Game/Blueprints/Slime/Spawning/SpawnBounds` _output_get)) (`local.AreaPerPoint`))) 1))
      (`KismetArrayLibrary.Array_Add` (`local.OutPoints`) (`KismetMathLibrary.RandomPointInBoundingBox` _currentspawnbounds_origin _currentspawnbounds_bounds))))
  (return (`local.OutPoints`)))

(fn `UserConstructionScript`)