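; BP_Special is a player special ability with activation gating and a cooldown, apparently meant as a base for specific specials.
; AttemptToActivate calls Activate only when CanActivate finds IsActive false, and Activate sets that flag.
; FinishActivate starts a one-shot Cooldown timer.
; FinishCooldown clears IsActive and broadcasts OnCanActivate, so the flag covers both the active and cooldown phases.
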(fn `Activate`
  (set `self.IsActive` true)
  (return))

(fn `AttemptToActivate`
  (if (`self.CanActivate`)
    (`self.Activate`))
  (return))

(fn `CanActivate`
  (returns (ReturnValue :type Boolean))
  (return (not (`self.IsActive`))))

(fn `FinishActivate`
  (`KismetSystemLibrary.K2_SetTimerDelegate` (`|CreateDelegate` :!event `FinishCooldown`) (`self.Cooldown`))
  (return))

(fn `FinishCooldown`
  (set `self.IsActive` false)
  (`self.OnCanActivate`)
  (return))

(fn `UserConstructionScript`)