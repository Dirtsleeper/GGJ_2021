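; Blueprint function library that looks up the colors and icon for each slime color type.
; GetSlimeColor builds parameter names from the enum's string and reads base, inlight and directional light colors from the MPC_SlimeColor material parameter collection, so each enum value relies on matching parameter names.
; GetSlimeIcon maps the slime type to an icon through a Select, with Bronze, Silver and Gold left unassigned.
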(fn `GetSlimeColor`
  (params (ColorIn :type "/Game/Blueprints/Slime/ESlimeColor Enum" :default "NewEnumerator0"))
  (returns (BaseColor :type "LinearColor Structure") (InlightColor :type "LinearColor Structure") (DirectionalLightColor :type "LinearColor Structure"))
  (bind _returnvalue (`KismetMaterialLibrary.GetVectorParameterValue` (`local.__WorldContext`) "/Game/Blueprints/Slime/MPC_SlimeColor.MPC_SlimeColor" (`KismetStringLibrary.Conv_StringToName` (`KismetTextLibrary.Conv_TextToString` (`|FormatText` "DirectionalLightColor_{Color}" (`|GetEnumeratorNameAsString` ColorIn))))))
  (bind _returnvalue_2 (`KismetMaterialLibrary.GetVectorParameterValue` (`local.__WorldContext`) "/Game/Blueprints/Slime/MPC_SlimeColor.MPC_SlimeColor" (`KismetStringLibrary.Conv_StringToName` (`KismetTextLibrary.Conv_TextToString` (`|FormatText` "InlightColor_{Color}" (`|GetEnumeratorNameAsString` (`local.ColorIn`)))))))
  (bind _returnvalue_3 (`KismetMaterialLibrary.GetVectorParameterValue` (`local.__WorldContext`) "/Game/Blueprints/Slime/MPC_SlimeColor.MPC_SlimeColor" (`KismetStringLibrary.Conv_StringToName` (`KismetTextLibrary.Conv_TextToString` (`|FormatText` "BaseColor_{Color}" (`|GetEnumeratorNameAsString` (`local.ColorIn`)))))))
  (return _returnvalue_3 _returnvalue_2 _returnvalue))

(fn `GetSlimeIcon`
  (params (Slime :type "/Game/Blueprints/Slime/ESlimeColor Enum" :default "NewEnumerator0"))
  (returns (ReturnValue :type "Texture2D Object Reference"))
  (return (select `/Game/Blueprints/Slime/ESlimeColor` Slime :`NewEnumerator0` "/Game/Assets/UI/Icons/SLIME_CLR10.SLIME_CLR10" :`NewEnumerator1` "/Game/Assets/UI/Icons/SLIME_CLR7.SLIME_CLR7" :`NewEnumerator2` "/Game/Assets/UI/Icons/SLIME_CLR6.SLIME_CLR6" :`NewEnumerator3` "/Game/Assets/UI/Icons/SLIME_CLR3.SLIME_CLR3" :`NewEnumerator4` "/Game/Assets/UI/Icons/SLIME_CLR4.SLIME_CLR4" :`NewEnumerator5` "/Game/Assets/UI/Icons/SLIME_CLR14.SLIME_CLR14" :`NewEnumerator9` "/Game/Assets/UI/Icons/SLIME_CLR1.SLIME_CLR1" :!type "Texture2D Object Reference")))