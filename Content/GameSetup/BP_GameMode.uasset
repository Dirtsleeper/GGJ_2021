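; Game mode for a four-player local split-screen game that sets up players and holds the value of each slime color.
; BeginPlay enables split screen, then gets or creates four player controllers, sets their input mode and restarts each at its index-named player start.
; New players are collected in a controller array.
; A color-to-value map is supplied externally, triggers a game-initialized call and defaults to 1 on failed lookups.
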(event `self.ReceiveBeginPlay`
  (`self.ToggleSplitScreen` true)
  (`self.InitializePlayers`))

(event `self.HandleStartingNewPlayer`
  (params (NewPlayer :type "PlayerController Object Reference"))
  (`KismetArrayLibrary.Array_Add` (`self.PlayerControllers`) NewPlayer))

(fn `GetSlimeValue`
  (params (Color :type "/Game/Blueprints/Slime/ESlimeColor Enum" :default "NewEnumerator0"))
  (returns (Value :type Integer))
  (bind (_value _returnvalue) (`BlueprintMapLibrary.Map_Find` (`self.SlimeValue`) Color))
  (if _returnvalue
    (return _value)
    (else
      (return 1))))

(fn `InitializePlayers`
  (locals (CurrentController :type "PlayerController Object Reference"))
  (bind _currentcontroller (`local.CurrentController`))
  (for _index (range 4)
    (bind _returnvalue (`GameplayStatics.GetPlayerController` _index))
    (`/Engine/EditorBlueprintResources/StandardMacros.IsValid` _returnvalue
      (:`Is Valid`
        (set `local.CurrentController` _returnvalue))
      (:`Is Not Valid`
        (bind _returnvalue_2 (`GameplayStatics.CreatePlayer` -1))
        (set `local.CurrentController` _returnvalue_2)))
    (`WidgetBlueprintLibrary.SetInputMode_GameAndUIEx` (`local.CurrentController`) null)
    (bind _returnvalue_3 (`self.K2_FindPlayerStart` _currentcontroller (`KismetStringLibrary.Concat_StrStr` "Player" (`KismetStringLibrary.Conv_IntToString` _index))))
    (`/Engine/EditorBlueprintResources/StandardMacros.IsValid` _returnvalue_3
      (:`Is Valid`
        (`self.RestartPlayerAtPlayerStart` _currentcontroller _returnvalue_3)))))

(fn `InitializeSlimeValue`
  (params (NewSlimeValues :type "Map of /Game/Blueprints/Slime/ESlimeColor Enum to Integer"))
  (set `self.SlimeValue` NewSlimeValues)
  (`self.OnGameInitialized`)
  (return))

(fn `UserConstructionScript`)