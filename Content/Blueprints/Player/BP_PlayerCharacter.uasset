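; Player character that picks up slimes, carries them in a sack and turns them in to a King Slime.
; Interaction targets the nearest slime pawn within a facing angle; walk speed scales down as the sack's gamemode-valued count grows.
; A dash actor spawned and attached on BeginPlay serves as the special ability.
; Attacks are unfinished: RecieveAttack runs on the attacker itself, only prints stun and drop messages, and the drop calculation is a stub.
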(event `self.ReceiveBeginPlay`
  (`parent.ReceiveBeginPlay`)
  (bind _returnvalue (`|SpawnActorFromClass` "/Game/Blueprints/Player/Specials/BP_Dash.BP_Dash_C" (`KismetMathLibrary.MakeTransform` (`self.K2_GetActorLocation`)) "Undefined" "OverrideRootScale" self self null))
  (bind _output_get (set `self.MySpecial` _returnvalue))
  (`self.K2_AttachToActor` _output_get self "None" "SnapToTarget" "KeepRelative" "KeepRelative" true))

(fn `AddCollectedSlimes`
  (params (Slimes :type "Map of /Game/Blueprints/Slime/ESlimeColor Enum to Integer"))
  (locals (CurrentColor :type "/Game/Blueprints/Slime/ESlimeColor Enum"))
  (bind _keys (`BlueprintMapLibrary.Map_Keys` Slimes))
  (for _array_element _keys
    (set `local.CurrentColor` _array_element)
    (`BlueprintMapLibrary.Map_Add` (`self.CollectedInventory`) (`local.CurrentColor`) (+ (`BlueprintMapLibrary.Map_Find` (`local.Slimes`) (`local.CurrentColor`)) (`BlueprintMapLibrary.Map_Find` (`self.CollectedInventory`) (`local.CurrentColor`)))))
  (return))

(fn `AddSlimeToSack`
  (params (SlimeColor :type "/Game/Blueprints/Slime/ESlimeColor Enum" :default "NewEnumerator0"))
  (locals (SlimeValue :type Integer :default 0))
  (bind _slimesackinventory (`self.SlimeSackInventory`))
  (bind _asbp_gamemode (cast `/Game/GameSetup/BP_GameMode` (`GameplayStatics.GetGameMode`)))
  (set `local.SlimeValue` (`/Game/GameSetup/BP_GameMode.GetSlimeValue` _asbp_gamemode SlimeColor))
  (`BlueprintMapLibrary.Map_Add` _slimesackinventory (`local.SlimeColor`) (+ (`BlueprintMapLibrary.Map_Find` _slimesackinventory (`local.SlimeColor`)) (`local.SlimeValue`)))
  (`self.ModifySlimeCount` (`local.SlimeValue`)))

(fn `AttemptActivateSpecial`
  (`/Game/Blueprints/Player/Specials/BP_Special.AttemptToActivate` (`self.MySpecial`))
  (return))

(fn `CalculateSlimeToDrop`
  (params (Attacker :type "/Game/Blueprints/Player/BP_PlayerCharacter Object Reference"))
  (returns (DroppedSlime :type Integer))
  ;[1 1 1] Talk math with Casey
)

(fn `ClearSlimeSack`
  (`BlueprintMapLibrary.Map_Clear` (`self.SlimeSackInventory`))
  (bind _output_get (set `self.SackSlimeCount` 0))
  (`self.OnSlimeCountModified` _output_get)
  (`self.UpdateMovementSpeed`)
  (return))

(fn `GetAllActorsInAngle`
  (params (ActorClass :type "Actor Class Reference") (Angle :type "Float (double-precision)") (SortByDistance :type Boolean))
  (returns (Actors :type "Array of Actor Object Reference"))
  (locals (ClosestActorDistance :type "Float (double-precision)") (ClosestActor :type "Actor Object Reference") (ActorsInRange :type "Array of Actor Object Reference") (ActorDistanceMap :type "Map of Actor Object Reference to Float (double-precision)"))
  (bind (_returnvalue_roll _returnvalue_pitch _returnvalue_yaw) (`KismetMathLibrary.BreakRotator` (`self.K2_GetActorRotation`)))
  (bind _closestactor (`local.ClosestActor`))
  (for _array_element (`PrimitiveComponent.GetOverlappingActors` (`self.InteractCollider`) ActorClass)
    (if SortByDistance
      (bind (_returnvalue_roll_2 _returnvalue_pitch_2 _returnvalue_yaw_2) (`KismetMathLibrary.BreakRotator` (`KismetMathLibrary.FindLookAtRotation` (`self.K2_GetActorLocation`) (`self.K2_GetActorLocation` _array_element))))
      (if (<= (`KismetMathLibrary.Abs` (- _returnvalue_yaw_2 _returnvalue_yaw)) (/ (`local.Angle`) 2.0))
        (`BlueprintMapLibrary.Map_Add` (`local.ActorDistanceMap`) _array_element (`self.GetDistanceTo` _array_element self)))
      (else
        (`KismetArrayLibrary.Array_Add` (`local.ActorsInRange`) _array_element))))
  (if SortByDistance
    (while (!= (`BlueprintMapLibrary.Map_Length` (`local.ActorDistanceMap`)) 0)
      (set `local.ClosestActor` null)
      (bind _keys (`BlueprintMapLibrary.Map_Keys` (`local.ActorDistanceMap`)))
      (for _array_element_2 _keys
        (bind _value (`BlueprintMapLibrary.Map_Find` (`local.ActorDistanceMap`) _array_element_2))
        (if (or (< _value (`local.ClosestActorDistance`)) (not (`KismetSystemLibrary.IsValid` (`local.ClosestActor`))))
          (set `local.ClosestActor` _array_element_2)
          (set `local.ClosestActorDistance` _value)))
      (`KismetArrayLibrary.Array_Add` (`local.ActorsInRange`) _closestactor)
      (`BlueprintMapLibrary.Map_Remove` (`local.ActorDistanceMap`) _closestactor))
    (return (`local.ActorsInRange`))
    (else
      (return (`local.ActorsInRange`)))))

(fn `GetInventory`
  (returns (Inventory :type "Map of /Game/Blueprints/Slime/ESlimeColor Enum to Integer"))
  (return (`self.CollectedInventory`)))

(fn `HandleAttack`
  (for _array_element (`PrimitiveComponent.GetOverlappingActors` (`self.InteractCollider`) "BP_PlayerCharacter_C")
    (bind _asbp_player_character (cast `/Game/Blueprints/Player/BP_PlayerCharacter` _array_element))
    (if (!= _asbp_player_character self)
      (`self.Recieve Attack` self))))

(fn `HandleInteract`
  (locals (MaximumInteractAngle :type "Float (double-precision)" :default 90.0) (OutActors :type "Array of Actor Object Reference"))
  (bind _output (`|GetArrayItem` (`local.OutActors`)))
  (bind _output_get (set `local.OutActors` (`self.GetAllActorsInAngle` "/Game/Blueprints/Slime/BP_SlimePawn.BP_SlimePawn_C" (`local.MaximumInteractAngle`) true)))
  (if (> (`KismetArrayLibrary.Array_Length` _output_get) 0)
    (bind _asbp_slime (cast `/Game/Blueprints/Slime/BP_Slime` _output)
      (:`then`
        (`self.PickupSlime` _asbp_slime))
      (:`CastFailed`
        (bind _asbp_king_slime (cast `/Game/Blueprints/Slime/BP_KingSlime` _output))
        (`/Game/Blueprints/Slime/BP_KingSlime.TurnInSlimes` _asbp_king_slime self)))))

(fn `ModifySlimeCount`
  (params (Amount :type Integer))
  (bind _output_get (set `self.SackSlimeCount` (+ Amount (`self.SackSlimeCount`))))
  (`self.OnSlimeCountModified` _output_get)
  (`self.UpdateMovementSpeed`))

(fn `PickupSlime`
  (params (Slime :type "/Game/Blueprints/Slime/BP_Slime Object Reference"))
  (`/Game/Blueprints/Slime/BP_Slime.OnPickup` Slime self)
  (`ActorComponent.SetActive` (`self.GetMovementComponent`) false false)
  (return))

(fn `Recieve Attack`
  (params (Attacker :type "/Game/Blueprints/Player/BP_PlayerCharacter Object Reference"))
  (`KismetSystemLibrary.PrintString` (`KismetStringLibrary.Concat_StrStr` (`KismetSystemLibrary.GetDisplayName` self) "Is Stunned!"))
  (bind _droppedslime (`self.CalculateSlimeToDrop` Attacker))
  (`KismetSystemLibrary.PrintString` (`KismetStringLibrary.Concat_StrStr` (`KismetStringLibrary.Conv_IntToString` _droppedslime) "Slimes where Dropped!")))

(fn `UpdateMovementSpeed`
  (set `CharacterMovementComponent.MaxWalkSpeed` (`KismetMathLibrary.MapRangeClamped` (`KismetMathLibrary.Conv_IntToDouble` (`self.SackSlimeCount`)) 0.0 20.0 (`self.MaxWalkSpeed`)) (`self.CharacterMovement`)))

(fn `UserConstructionScript`)