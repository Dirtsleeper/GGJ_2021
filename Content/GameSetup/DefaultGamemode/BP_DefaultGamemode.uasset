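; Default game mode that tracks the shared slime score per color against target totals.
; CalculateTargetScore sets a fixed target for three colors and broadcasts OnGameInitialized.
; TurnInSlimes adds a player's slimes to the current score, clamped to each target, and records the amount awarded minus any overflow.
; It broadcasts OnScoreChanged when the awarded map has entries, and GetScore exposes the running totals.
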(event `self.ReceiveBeginPlay`)

(fn `CalculateTargetScore`
  (`BlueprintMapLibrary.Map_Add` (`self.TargetScore`) "NewEnumerator0" 10)
  (`BlueprintMapLibrary.Map_Add` (`self.TargetScore`) "NewEnumerator2" 10)
  (`BlueprintMapLibrary.Map_Add` (`self.TargetScore`) "NewEnumerator1" 10)
  (`self.OnGameInitialized`))

(fn `GetScore`
  (returns (Current :type "Map of /Game/Blueprints/Slime/ESlimeColor Enum to Integer"))
  (return (`self.CurrentScore`)))

(fn `TurnInSlimes`
  (params (Player :type "/Game/Blueprints/Player/BP_PlayerCharacter Object Reference") (Slimes :type "Map of /Game/Blueprints/Slime/ESlimeColor Enum to Integer"))
  (locals (Max :type Integer) (GameTotal :type Integer) (PlayerScore :type Integer) (Color :type "/Game/Blueprints/Slime/ESlimeColor Enum") (SlimesAwarded :type "Map of /Game/Blueprints/Slime/ESlimeColor Enum to Object Object Reference"))
  (bind _returnvalue (+ (`local.GameTotal`) (`local.PlayerScore`)))
  (bind _keys (`BlueprintMapLibrary.Map_Keys` Slimes))
  (for _array_element _keys
    (set `local.Color` _array_element)
    (set `local.GameTotal` (`BlueprintMapLibrary.Map_Find` (`self.CurrentScore`) (`local.Color`)))
    (set `local.Max` (`BlueprintMapLibrary.Map_Find` (`self.TargetScore`) (`local.Color`)))
    (set `local.PlayerScore` (`BlueprintMapLibrary.Map_Find` (`local.Slimes`) (`local.Color`)))
    (`BlueprintMapLibrary.Map_Add` (`self.CurrentScore`) (`local.Color`) (`KismetMathLibrary.Clamp` _returnvalue 0 (`local.Max`)))
    (`BlueprintMapLibrary.Map_Add` (`local.SlimesAwarded`) (`local.Color`) (- (`local.PlayerScore`) (`KismetMathLibrary.Max` (- _returnvalue (`local.Max`))))))
  (if (> (`BlueprintMapLibrary.Map_Length` (`local.SlimesAwarded`)) 0)
    (`self.OnScoreChanged`))
  (return))

(fn `UserConstructionScript`
  (`parent.UserConstructionScript`))