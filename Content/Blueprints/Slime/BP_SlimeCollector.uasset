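; BP_SlimeCollector is a short-lived projectile that flies to a target player and credits them with slime.
; After a brief delay it homes on the player's SlimeTarget component, and it is destroyed on overlapping their mesh or when its lifespan expires.
; On destruction it adds the gamemode's value for its color to the player's slime count and reactivates the player's movement component.
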(event `self.ReceiveBeginPlay`
  (`parent.ReceiveBeginPlay`)
  (set `ProjectileMovementComponent.HomingTargetComponent` (`/Game/Blueprints/Player/BP_PlayerCharacter.SlimeTarget` (`self.TargetPlayer`)) (`self.ProjectileMovement`))
  (`KismetSystemLibrary.Delay` 0.3)
  (set `ProjectileMovementComponent.bIsHomingProjectile` true (`self.ProjectileMovement`))
  (`self.SetLifeSpan` 0.6))

(event `self.ReceiveDestroyed`
  (bind _asbp_gamemode (cast `/Game/GameSetup/BP_GameMode` (`GameplayStatics.GetGameMode`)))
  (`/Game/Blueprints/Player/BP_PlayerCharacter.ModifySlimeCount` (`self.TargetPlayer`) (`/Game/GameSetup/BP_GameMode.GetSlimeValue` _asbp_gamemode (`self.MyColor`)))
  (`ActorComponent.SetActive` (`Pawn.GetMovementComponent` (`self.TargetPlayer`)) true false))

(event `self.Sphere.OnComponentBeginOverlap`
  (params (OverlappedComponent :type "PrimitiveComponent Object Reference") (OtherActor :type "Actor Object Reference") (OtherComp :type "PrimitiveComponent Object Reference") (OtherBodyIndex :type Integer) (bFromSweep :type Boolean) (SweepResult :type "HitResult Structure (by ref)"))
  (bind _targetplayer (`self.TargetPlayer`))
  (`KismetSystemLibrary.PrintString` "Overlap")
  (if (and (== OtherActor _targetplayer) (== OtherComp (`Character.Mesh` _targetplayer)))
    (`self.K2_DestroyActor`)))

(fn `UserConstructionScript`)