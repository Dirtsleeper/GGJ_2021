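; Player controller for the main menu lobby, giving each local player menu focus and letting the first player start the game.
; InitializeHUD sets user focus on the play button of the lobby player card matching this controller's ID.
; Gamepad Special Right on controller 0 runs AttemptToStartGame, which checks lobby readiness and has the game instance load a map with the lobby's player count.
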(event `Key|Gamepad_Special_Right`
  (params (Key :type "Key Structure"))
  (:`Pressed`
    (if (== (`GameplayStatics.GetPlayerControllerID` self) 0)
      (`self.AttemptToStartGame`))))

(fn `AttemptToStartGame`
  (bind _asbp_main_menu_gamemode (cast `/Game/GameSetup/MainMenu/BP_MainMenuGamemode` (`GameplayStatics.GetGameMode`)))
  (bind _lobbymenu (`/Game/GameSetup/MainMenu/BP_MainMenuHUD.LobbyMenu` (`/Game/GameSetup/MainMenu/BP_MainMenuGamemode.MainMenuHUD` _asbp_main_menu_gamemode)))
  (if (`/Game/HUD/Lobby/BPW_Lobby.IsReadyToBegin` _lobbymenu)
    (bind _asbp_game_instance (cast `/Game/GameSetup/BP_GameInstance` (`GameplayStatics.GetGameInstance`)))
    (`/Game/GameSetup/BP_GameInstance.LoadMap` _asbp_game_instance "NewEnumerator1" (`/Game/HUD/Lobby/BPW_Lobby.GetNumPlayers` _lobbymenu))))

(fn `InitializeHUD`
  (bind _asbp_main_menu_gamemode (cast `/Game/GameSetup/MainMenu/BP_MainMenuGamemode` (`GameplayStatics.GetGameMode`)))
  (`Widget.SetUserFocus` (`/Game/HUD/Lobby/BPW_PlayerCard.PlayButton` (`/Game/HUD/Lobby/BPW_Lobby.GetPlayerCard` (`/Game/GameSetup/MainMenu/BP_MainMenuHUD.LobbyMenu` (`/Game/GameSetup/MainMenu/BP_MainMenuGamemode.MainMenuHUD` _asbp_main_menu_gamemode)) (`GameplayStatics.GetPlayerControllerID` self))) self))

(fn `UserConstructionScript`)