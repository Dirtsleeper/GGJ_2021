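; Player controller that translates input into pawn movement, camera look, character actions and HUD control.
; Movement axes are stored and applied along the pawn's forward and right vectors, and yaw input only applies while its movement component is active.
; Interact, Attack and Special forward to handlers on BP_PlayerCharacter.
; OpenSlimeSack toggles the HUD's slime sack widget on both press and release, giving hold-to-view behavior.
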(event `InputAxis|MoveForward`
  (params (AxisValue :type "Float (single-precision)"))
  (bind _returnvalue (`self.K2_GetPawn`))
  (bind _output_get (set `self.MyMoveForwardAxis` AxisValue))
  (`Pawn.AddMovementInput` _returnvalue (`self.GetActorForwardVector` _returnvalue) _output_get false))

(event `InputAxis|MoveRight`
  (params (AxisValue :type "Float (single-precision)"))
  (bind _returnvalue (`self.K2_GetPawn`))
  (bind _output_get (set `self.MyMoveRightAxis` AxisValue))
  (`Pawn.AddMovementInput` _returnvalue (`self.GetActorRightVector` _returnvalue) _output_get false))

(event `InputAxis|LookUp`
  (params (AxisValue :type "Float (single-precision)"))
  (`Pawn.AddControllerPitchInput` (`self.K2_GetPawn`) AxisValue))

(event `InputAxis|LookRight`
  (params (AxisValue :type "Float (single-precision)"))
  (bind _returnvalue (`self.K2_GetPawn`))
  (if (`ActorComponent.IsActive` (`Pawn.GetMovementComponent` _returnvalue))
    (`Pawn.AddControllerYawInput` _returnvalue AxisValue)))

(event `InputAction|Interact`
  (params (Key :type "Key Structure"))
  (:`Pressed`
    (bind _asbp_player_character (cast `/Game/Blueprints/Player/BP_PlayerCharacter` (`self.K2_GetPawn`)))
    (`/Game/Blueprints/Player/BP_PlayerCharacter.HandleInteract` _asbp_player_character)))

(event `InputAction|Attack`
  (params (Key :type "Key Structure"))
  (:`Pressed`
    (bind _asbp_player_character (cast `/Game/Blueprints/Player/BP_PlayerCharacter` (`self.K2_GetPawn`)))
    (`/Game/Blueprints/Player/BP_PlayerCharacter.HandleAttack` _asbp_player_character)))

(event `InputAction|Special`
  (params (Key :type "Key Structure"))
  (:`Pressed`
    (bind _asbp_player_character (cast `/Game/Blueprints/Player/BP_PlayerCharacter` (`self.K2_GetPawn`)))
    (`/Game/Blueprints/Player/BP_PlayerCharacter.AttemptActivateSpecial` _asbp_player_character)))

(event `InputAction|OpenSlimeSack`
  (params (Key :type "Key Structure"))
  (:`Pressed`
    (bind _asbp_default_gamemode_hud (cast `/Game/GameSetup/DefaultGamemode/BP_DefaultGamemodeHUD` (`self.GetHUD`) :!label _label))
    (`/Game/HUD/Player/BPW_SlimeSack.ToggleVisibility` (`/Game/HUD/Player/BPW_PlayerHUD.SlimeSack` (`/Game/GameSetup/DefaultGamemode/BP_DefaultGamemodeHUD.MyHUDWidget` _asbp_default_gamemode_hud))))
  (:`Released`
    (goto _label)))

(fn `UserConstructionScript`)